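; BP_MeteorProjectile is a mage projectile that deals area damage as a meteor when it hits.
; On a hit, only the authority applies radial damage with falloff around its location, ignoring the instigator and crediting that instigator's controller.
; Its construction script runs the parent's setup, then assigns the meteorite mesh at enlarged scale and sets the projectile movement's initial and maximum speeds from variables.
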(event EventHit
  (params (MyComp :type Primitive%20Component%20Object%20Reference) (Other :type Actor%20Object%20Reference) (OtherComp :type Primitive%20Component%20Object%20Reference) (bSelfMoved :type Boolean) (HitLocation :type Vector :default "0, 0, 0") (HitNormal :type Vector :default "0, 0, 0") (NormalImpulse :type Vector :default "0, 0, 0") (Hit :type Hit%20Result%20Structure%20%28by%20ref%29))
  (bind _instigator (Variables|Default|GetInstigator))
  (Networking|SwitchHasAuthority
    (:Authority
      (Class|GameplayStatics|ApplyRadialDamagewithFalloff 0 (Variables|Default|GetDamage) (Variables|Projectile|GetMinDamage) (Transformation|GetActorLocation) 1e+02 4e+02 5.0 (Variables|Default|GetDamage%20Type) (Utilities|Array|MakeArray _instigator) self (Game|GetInstigatorController _instigator) "ECC_Visibility"))))

(fn ConstructionScript
  (bind _projectilemovement (Variables|Default|GetProjectileMovement))
  (|CallParentFunction)
  (Components|StaticMesh|SetStaticMesh "/Game/Characters/Mage/Projectiles/Meshes/Meteorite.Meteorite")
  (Variables|/Script/Engine.ProjectileMovementComponent|SetInitialSpeed _projectilemovement (Variables|Projectile|GetInitial%20Speed))
  (Variables|/Script/Engine.ProjectileMovementComponent|SetMaxSpeed _projectilemovement (Variables|Projectile|GetMax%20Speed))
  (Transformation|SetWorldScale3D (Variables|Default|GetProjectileMesh) "2.000000,2.000000,2.000000"))