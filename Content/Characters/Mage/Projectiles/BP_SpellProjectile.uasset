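; Spell projectile for the Mage that damages the actor it hits, using its Damage and DamageType variables and crediting the instigator's controller.
; Hit handling runs only on authority, which applies the damage, then hides the projectile, disables its collision and sets a short lifespan instead of destroying it immediately.
; The construction script makes the collision component ignore the instigator when moving, so the projectile passes through its caster.
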(event EventHit
  (params (MyComp :type Primitive%20Component%20Object%20Reference) (Other :type Actor%20Object%20Reference) (OtherComp :type Primitive%20Component%20Object%20Reference) (bSelfMoved :type Boolean) (HitLocation :type Vector :default "0, 0, 0") (HitNormal :type Vector :default "0, 0, 0") (NormalImpulse :type Vector :default "0, 0, 0") (Hit :type Hit%20Result%20Structure%20%28by%20ref%29))
  (Networking|SwitchHasAuthority
    (:Authority
      (Game|Damage|ApplyDamage Other (Variables|Projectile|GetDamage) (Game|GetInstigatorController (Variables|Actor|GetInstigator)) self (Variables|Projectile|GetDamage%20Type))
      (Actor|SetLifeSpan 2.0)
      (Rendering|SetActorHiddenInGame true)
      (Collision|SetActorEnableCollision false))))

(fn ConstructionScript
  (Collision|IgnoreActorwhenMoving (Variables|Projectile|GetCollisionComp) (Game|GetInstigator) true))